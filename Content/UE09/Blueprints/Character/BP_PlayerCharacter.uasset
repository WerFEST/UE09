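; BP_PlayerCharacter is a player character Blueprint that handles opening the inventory and interacting with world objects.
; Pressing I creates a new inventory widget, adds it to the viewport and has its grid display the BACInventorySystem inventory.
; Pressing E takes a short-range aim point hit and sends InteractMessage, passing itself, to any hit actor implementing BPI_Interactable.
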(event EventBeginPlay)

(event Input|KeyboardEvents|I
  (params (Key :type Key%20Structure :default "None"))
  (:Pressed
    (bind _returnvalue (UserInterface|CreateWidget "/Game/UE09/Widgets/Inventory/W_Intentory.W_Intentory_C" (Game|GetPlayerController 0)))
    (UserInterface|Viewport|AddtoViewport _returnvalue 0)
    (Default|DisplayInventory (Variables|/Game/UE09/Widgets/Inventory/W_Intentory.W_Intentory_C|GetWBP_InventoryGrid _returnvalue) (Variables|Default|GetBAC_InventorySystem))))

(event Input|KeyboardEvents|E
  (params (Key :type Key%20Structure :default "None"))
  (bind _hitresult (Class|UE09BaseCharacter|GetAimPoint 5e+02))
  (bind (_bblockinghit _binitialoverlap _time _distance _location _impactpoint _normal _impactnormal _physmat _hitactor) (Collision|BreakHitResult _hitresult))
  (:Pressed
    (if _bblockinghit
      (if (Utilities|DoesObjectImplementInterface _hitactor "/Game/UE09/Blueprints/Interfaces/BPI_Interactable.BPI_Interactable_C")
        (Class|BPIInteractable|Interact(Message) _hitactor self)))))

(fn ConstructionScript)