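; BP_BaseItem is a base world item actor that can be picked up into an interacting actor's inventory.
; On BeginPlay it copies its Quantity into its BACItemInventory component, which holds the item's data row.
; Interact looks for a BAC_InventorySystem component on the interactor and adds the item by row name and quantity.
; The actor destroys itself on success; otherwise it keeps the returned remaining quantity.
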(event EventBeginPlay
  (Variables|/Game/UE09/Blueprints/Components/Inventory/BAC_ItemInventory.BAC_ItemInventory_C|SetQuantity (Variables|Default|GetBAC_ItemInventory) (Variables|Default|GetQuantity)))

(event EventInteract
  (params (Actor :type Actor%20Object%20Reference))
  (bind _returnvalue (Actor|GetComponentbyClass Actor "/Game/UE09/Blueprints/Components/Inventory/BAC_InventorySystem.BAC_InventorySystem_C"))
  (bind _bac_iteminventory (Variables|Default|GetBAC_ItemInventory))
  (Utilities|IsValid _returnvalue
    (:Is%20Valid
      (bind (_bissuccess _quanityremain) (Default|AddtoInventory _returnvalue (.rowname (Variables|/Game/UE09/Blueprints/Components/Inventory/BAC_ItemInventory.BAC_ItemInventory_C|GetItemData _bac_iteminventory)) (Variables|/Game/UE09/Blueprints/Components/Inventory/BAC_ItemInventory.BAC_ItemInventory_C|GetQuantity _bac_iteminventory)))
      (if _bissuccess
        (Actor|DestroyActor)
        (else
          (Variables|/Game/UE09/Blueprints/Components/Inventory/BAC_ItemInventory.BAC_ItemInventory_C|SetQuantity (Variables|Default|GetBAC_ItemInventory) _quanityremain))))))

(fn ConstructionScript)